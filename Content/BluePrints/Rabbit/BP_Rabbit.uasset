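; BP_Rabbit is a character that chases the player whenever both share the same CurrentFloor value.
; BeginPlay caches the player as Target, and Tick smoothly turns the rabbit's yaw toward it and moves it forward with direct movement input.
; Capsule hits call Destruct on any WoodenBox it runs into.
; A ToggleCrouch event flip-flops between crouching and standing.
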(event `ToggleCrouch`
  (`/Engine/EditorBlueprintResources/StandardMacros.FlipFlop`
    (:`A`
      (`self.Crouch`)
      (set `self.Crouching` true))
    (:`B`
      (`self.UnCrouch`)
      (set `self.Crouching` false))))

(event `self.ReceiveBeginPlay`
  (bind _asplayer_character (cast `/Game/BluePrints/PlayerCharacter` (`GameplayStatics.GetPlayerPawn` 0)))
  (set `self.Target` _asplayer_character))

(event `self.ReceiveTick`
  (params (DeltaSeconds :type "Float (single-precision)"))
  (set `self.DeltaTime` DeltaSeconds)
  (if (== (`/Game/BluePrints/PlayerCharacter.CurrentFloor` (stale `self.ReceiveBeginPlay` _asplayer_character)) (`self.CurrentFloor`))
    (`self.K2_SetActorRotation` (`KismetMathLibrary.RInterpTo` (`self.K2_GetActorRotation`) (`KismetMathLibrary.MakeRotator` 0.0 0.0 (.yaw (`KismetMathLibrary.FindLookAtRotation` (`self.K2_GetActorLocation`) (`self.K2_GetActorLocation` (`self.Target`))))) (`self.DeltaTime`)))
    (`self.AddMovementInput` (`KismetMathLibrary.GetForwardVector` (`self.K2_GetActorRotation`)))))

(event `self.CapsuleComponent.OnComponentHit`
  (params (HitComponent :type "PrimitiveComponent Object Reference") (OtherActor :type "Actor Object Reference") (OtherComp :type "PrimitiveComponent Object Reference") (NormalImpulse :type "Vector Structure") (Hit :type "HitResult Structure (by ref)"))
  (if (== OtherActor (cast `/Game/BluePrints/Props/WoodenBox` OtherActor :!pure true))
    (bind _aswooden_box (cast `/Game/BluePrints/Props/WoodenBox` OtherActor))
    (`/Game/BluePrints/Props/WoodenBox.Destruct` _aswooden_box)))

(fn `UserConstructionScript`)