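; Ladder actor that moves the player between its top and bottom ends by teleporting rather than climbing.
; Upper and lower trigger boxes set the current and target sides and toggle the player character's ladder-availability flag on overlap.
; While available, Tick polls the character's Temp flag, then UseLadder snaps the player to the current side and, after a short delay, to the opposite side.
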(event `self.BoxUpperside.OnComponentBeginOverlap`
  (params (OverlappedComponent :type "PrimitiveComponent Object Reference") (OtherActor :type "Actor Object Reference") (OtherComp :type "PrimitiveComponent Object Reference") (OtherBodyIndex :type Integer) (bFromSweep :type Boolean) (SweepResult :type "HitResult Structure (by ref)"))
  (bind _returnvalue (`GameplayStatics.GetPlayerPawn` 0))
  (if (== OtherActor _returnvalue)
    (set `self.CurrentSide` (`self.Top`))
    (set `self.TargetSide` (`self.Bottom`))
    (bind _asplayer_character (cast `/Game/BluePrints/PlayerCharacter` _returnvalue))
    (bind _output_get (set `/Game/BluePrints/PlayerCharacter.IsAbleToUseLadder` true _asplayer_character))
    (set `self.IsAvailable` _output_get)
    (`KismetSystemLibrary.PrintString` "Can Use a Ladder" :!label _label)))

(event `self.BoxUpperside.OnComponentEndOverlap`
  (params (OverlappedComponent :type "PrimitiveComponent Object Reference") (OtherActor :type "Actor Object Reference") (OtherComp :type "PrimitiveComponent Object Reference") (OtherBodyIndex :type Integer))
  (bind _returnvalue (`GameplayStatics.GetPlayerPawn` 0))
  (if (== OtherActor _returnvalue)
    (bind _asplayer_character (cast `/Game/BluePrints/PlayerCharacter` _returnvalue))
    (bind _output_get (set `/Game/BluePrints/PlayerCharacter.IsAbleToUseLadder` false _asplayer_character))
    (set `self.IsAvailable` _output_get)
    (`KismetSystemLibrary.PrintString` "Can NOT Use a Ladder" :!label _label_2)))

(event `self.BoxUnderside.OnComponentBeginOverlap`
  (params (OverlappedComponent :type "PrimitiveComponent Object Reference") (OtherActor :type "Actor Object Reference") (OtherComp :type "PrimitiveComponent Object Reference") (OtherBodyIndex :type Integer) (bFromSweep :type Boolean) (SweepResult :type "HitResult Structure (by ref)"))
  (bind _returnvalue (`GameplayStatics.GetPlayerPawn` 0))
  (if (== OtherActor _returnvalue)
    (set `self.CurrentSide` (`self.Bottom`))
    (set `self.TargetSide` (`self.Top`))
    (bind _asplayer_character (cast `/Game/BluePrints/PlayerCharacter` _returnvalue))
    (bind _output_get (set `/Game/BluePrints/PlayerCharacter.IsAbleToUseLadder` true _asplayer_character))
    (set `self.IsAvailable` _output_get)
    (goto _label)))

(event `self.BoxUnderside.OnComponentEndOverlap`
  (params (OverlappedComponent :type "PrimitiveComponent Object Reference") (OtherActor :type "Actor Object Reference") (OtherComp :type "PrimitiveComponent Object Reference") (OtherBodyIndex :type Integer))
  (bind _returnvalue (`GameplayStatics.GetPlayerPawn` 0))
  (if (== OtherActor _returnvalue)
    (bind _asplayer_character (cast `/Game/BluePrints/PlayerCharacter` _returnvalue))
    (bind _output_get (set `/Game/BluePrints/PlayerCharacter.IsAbleToUseLadder` false _asplayer_character))
    (set `self.IsAvailable` _output_get)
    (goto _label_2)))

(event `self.ReceiveTick`
  (params (DeltaSeconds :type "Float (single-precision)"))
  (if (`self.IsAvailable`)
    (bind _asplayer_character (cast `/Game/BluePrints/PlayerCharacter` (`GameplayStatics.GetPlayerPawn` 0)))
    (if (`/Game/BluePrints/PlayerCharacter.Temp` _asplayer_character)
      (`self.UseLadder`)
      (set `/Game/BluePrints/PlayerCharacter.Temp` false _asplayer_character))))

(event `UseLadder`
  (bind _returnvalue (`SceneComponent.K2_GetComponentLocation` (`self.CurrentSide`)))
  (bind _returnvalue_2 (`SceneComponent.K2_GetComponentLocation` (`self.TargetSide`)))
  (bind _asplayer_character (cast `/Game/BluePrints/PlayerCharacter` (`GameplayStatics.GetPlayerPawn` 0)))
  (`self.K2_SetActorLocation` _asplayer_character _returnvalue false true)
  (`KismetSystemLibrary.PrintString` (`KismetStringLibrary.Conv_VectorToString` _returnvalue))
  (`KismetSystemLibrary.Delay` 0.5)
  (`self.K2_SetActorLocation` _asplayer_character _returnvalue_2 false true)
  (`KismetSystemLibrary.PrintString` (`KismetStringLibrary.Conv_VectorToString` _returnvalue_2)))

(fn `UserConstructionScript`)