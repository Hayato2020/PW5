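; PlayerCharacterController creates the player's inventory widget and keeps its text fields in sync with the inventory.
; BeginPlay creates UI_Inventory, loops over Inv indices to set the first three slot texts, and adds it to the viewport only on index 0.
; UpdateInv writes TakenKey to the fourth text field, then copies the first three Inv elements into the slot texts through an index switch.
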(event `self.ReceiveBeginPlay`
  (bind _text (`self.Text`))
  (bind _returnvalue (`|CreateWidget` "/Game/BluePrints/UI_inventory.UI_Inventory_C"))
  (for _index (range (+ (`KismetArrayLibrary.Array_Length` (`self.Inv`)) 1))
    (switch `int` _index
      (:`0`
        (set `/Game/BluePrints/UI_inventory.Text0` _text _returnvalue)
        (`UserWidget.AddToViewport` _returnvalue 0))
      (:`1`
        (set `/Game/BluePrints/UI_inventory.Text1` _text _returnvalue))
      (:`2`
        (set `/Game/BluePrints/UI_inventory.Text2` _text _returnvalue)))))

(event `UpdateInv`
  (set `/Game/BluePrints/UI_inventory.Text3` (`KismetTextLibrary.Conv_IntToText` (`self.TakenKey`)) (stale `self.ReceiveBeginPlay` _returnvalue))
  (for (_array_element _array_index) (`self.Inv`)
    (switch `int` _array_index
      (:`0`
        (bind _returnvalue (`KismetTextLibrary.Conv_ObjectToText` _array_element))
        (set `/Game/BluePrints/UI_inventory.Text0` _returnvalue (stale `self.ReceiveBeginPlay` _returnvalue)))
      (:`1`
        (set `/Game/BluePrints/UI_inventory.Text1` _returnvalue (stale `self.ReceiveBeginPlay` _returnvalue)))
      (:`2`
        (set `/Game/BluePrints/UI_inventory.Text2` _returnvalue (stale `self.ReceiveBeginPlay` _returnvalue))))))

(fn `UserConstructionScript`)