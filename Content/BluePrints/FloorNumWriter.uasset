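; FloorNumWriter is a trigger actor that records which floor the player or a rabbit is on.
; When something begins overlapping its Box, it writes its FloorNum into the CurrentFloor variable of that actor.
; The player pawn is handled as a PlayerCharacter, and any other actor is updated only if it casts to BP_Rabbit.
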(event `self.Box.OnComponentBeginOverlap`
  (params (OverlappedComponent :type "PrimitiveComponent Object Reference") (OtherActor :type "Actor Object Reference") (OtherComp :type "PrimitiveComponent Object Reference") (OtherBodyIndex :type Integer) (bFromSweep :type Boolean) (SweepResult :type "HitResult Structure (by ref)"))
  (if (== OtherActor (`GameplayStatics.GetPlayerPawn` 0))
    (bind _asplayer_character (cast `/Game/BluePrints/Player/PlayerCharacter` OtherActor))
    (set `/Game/BluePrints/Player/PlayerCharacter.CurrentFloor` (`self.FloorNum`) _asplayer_character)
    (else
      (bind _asbp_rabbit (cast `/Game/BluePrints/Rabbit/BP_Rabbit` OtherActor))
      (if (== _asbp_rabbit OtherActor)
        (set `/Game/BluePrints/Rabbit/BP_Rabbit.CurrentFloor` (`self.FloorNum`) _asbp_rabbit)))))

(fn `UserConstructionScript`)