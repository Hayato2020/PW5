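; Archetype Blueprint for a collectable item that the player picks up by walking into it.
; When its sphere overlaps the player pawn, it writes a reference to itself into the PlayerCharacterController's Inv array at the held-item count index.
; It then increments that count, calls UpdateInv and destroys itself, so the stored reference points to a destroyed actor.
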(event `self.Sphere1.OnComponentBeginOverlap`
  (params (OverlappedComponent :type "PrimitiveComponent Object Reference") (OtherActor :type "Actor Object Reference") (OtherComp :type "PrimitiveComponent Object Reference") (OtherBodyIndex :type Integer) (bFromSweep :type Boolean) (SweepResult :type "HitResult Structure (by ref)"))
  (if (== OtherActor (`GameplayStatics.GetPlayerPawn` 0))
    (bind _asplayer_character_controller (cast `/Game/BluePrints/PlayerCharacterController` (`GameplayStatics.GetPlayerController` 0)))
    (bind _numofholditems (`/Game/BluePrints/PlayerCharacterController.NumOfHoldItems` _asplayer_character_controller))
    (`KismetArrayLibrary.Array_Set` (`/Game/BluePrints/PlayerCharacterController.Inv` _asplayer_character_controller) _numofholditems self)
    (bind _result (`/Engine/EditorBlueprintResources/StandardMacros.IncrementInt` _numofholditems)
      (:`  `
        (set `/Game/BluePrints/PlayerCharacterController.NumOfHoldItems` _result _asplayer_character_controller)
        (`/Game/BluePrints/PlayerCharacterController.UpdateInv` _asplayer_character_controller)
        (`self.K2_DestroyActor`)))))

(fn `UserConstructionScript`)