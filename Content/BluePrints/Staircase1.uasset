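; Staircase ladder actor that lets the player trigger a climb, apparently unfinished.
; Upper and underside box overlaps toggle the character's IsAbleToUseLadder and set current/target sides, though only SceneUnderside is assigned; the other side is None.
; While available, Tick consumes the character's Temp flag to call UseLadder, which makes one VInterpTo step toward the current side.
; The timed teleport sequence through the middle to the target is disconnected.
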(event `self.BoxUpperside.OnComponentBeginOverlap`
  (params (OverlappedComponent :type "PrimitiveComponent Object Reference") (OtherActor :type "Actor Object Reference") (OtherComp :type "PrimitiveComponent Object Reference") (OtherBodyIndex :type Integer) (bFromSweep :type Boolean) (SweepResult :type "HitResult Structure (by ref)"))
  (bind _returnvalue (`GameplayStatics.GetPlayerPawn` 0))
  (if (== OtherActor _returnvalue)
    (set `self.CurrentSide` null)
    (set `self.TargetSide` (`self.SceneUnderside`))
    (bind _asplayer_character (cast `/Game/BluePrints/PlayerCharacter` _returnvalue))
    (bind _output_get (set `/Game/BluePrints/PlayerCharacter.IsAbleToUseLadder` true _asplayer_character))
    (set `self.IsAvailable` _output_get)
    (`KismetSystemLibrary.PrintString` "Can Use a Ladder" :!label _label)))

(event `self.BoxUpperside.OnComponentEndOverlap`
  (params (OverlappedComponent :type "PrimitiveComponent Object Reference") (OtherActor :type "Actor Object Reference") (OtherComp :type "PrimitiveComponent Object Reference") (OtherBodyIndex :type Integer))
  (bind _returnvalue (`GameplayStatics.GetPlayerPawn` 0))
  (if (== OtherActor _returnvalue)
    (bind _asplayer_character (cast `/Game/BluePrints/PlayerCharacter` _returnvalue))
    (bind _output_get (set `/Game/BluePrints/PlayerCharacter.IsAbleToUseLadder` false _asplayer_character))
    (set `self.IsAvailable` _output_get)
    (`KismetSystemLibrary.PrintString` "Can NOT Use a Ladder" :!label _label_2)))

(event `self.BoxUnderside.OnComponentBeginOverlap`
  (params (OverlappedComponent :type "PrimitiveComponent Object Reference") (OtherActor :type "Actor Object Reference") (OtherComp :type "PrimitiveComponent Object Reference") (OtherBodyIndex :type Integer) (bFromSweep :type Boolean) (SweepResult :type "HitResult Structure (by ref)"))
  (bind _returnvalue (`GameplayStatics.GetPlayerPawn` 0))
  (if (== OtherActor _returnvalue)
    (set `self.CurrentSide` (`self.SceneUnderside`))
    (set `self.TargetSide` null)
    (bind _asplayer_character (cast `/Game/BluePrints/PlayerCharacter` _returnvalue))
    (bind _output_get (set `/Game/BluePrints/PlayerCharacter.IsAbleToUseLadder` true _asplayer_character))
    (set `self.IsAvailable` _output_get)
    (goto _label)))

(event `self.BoxUnderside.OnComponentEndOverlap`
  (params (OverlappedComponent :type "PrimitiveComponent Object Reference") (OtherActor :type "Actor Object Reference") (OtherComp :type "PrimitiveComponent Object Reference") (OtherBodyIndex :type Integer))
  (bind _returnvalue (`GameplayStatics.GetPlayerPawn` 0))
  (if (== OtherActor _returnvalue)
    (bind _asplayer_character (cast `/Game/BluePrints/PlayerCharacter` _returnvalue))
    (bind _output_get (set `/Game/BluePrints/PlayerCharacter.IsAbleToUseLadder` false _asplayer_character))
    (set `self.IsAvailable` _output_get)
    (goto _label_2)))

(event `self.ReceiveTick`
  (params (DeltaSeconds :type "Float (single-precision)"))
  (bind _output_get (set `self.Delta Time` DeltaSeconds))
  (if (`self.IsAvailable`)
    (bind _asplayer_character (cast `/Game/BluePrints/PlayerCharacter` (`GameplayStatics.GetPlayerPawn` 0)))
    (if (`/Game/BluePrints/PlayerCharacter.Temp` _asplayer_character)
      (`self.UseLadder`)
      (set `/Game/BluePrints/PlayerCharacter.Temp` false _asplayer_character))))

(event `UseLadder`
  (bind _returnvalue (`SceneComponent.K2_GetComponentLocation` (`self.CurrentSide`)))
  (bind _asplayer_character (cast `/Game/BluePrints/PlayerCharacter` (`GameplayStatics.GetPlayerPawn` 0)))
  (`self.K2_SetActorLocation` _asplayer_character (`KismetMathLibrary.VInterpTo` (`SceneComponent.K2_GetComponentLocation` (`Character.Mesh` _asplayer_character)) _returnvalue (stale `self.ReceiveTick` _output_get) 1.0) false false)
  (`KismetSystemLibrary.PrintString` (`KismetStringLibrary.Conv_VectorToString` _returnvalue))
  (`KismetSystemLibrary.Delay` 1.0))

(fn `UserConstructionScript`)