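; LadderV2 is a climbable ladder volume for the player.
; When the player pawn begins overlapping its Box, the PlayerCharacter switches to Flying movement mode and its CanFly flag is set.
; When the overlap ends, movement returns to Walking and CanFly is cleared.
; The ladder itself only toggles this state and contains no climbing input or motion logic.
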(event `self.Box.OnComponentBeginOverlap`
  (params (OverlappedComponent :type "PrimitiveComponent Object Reference") (OtherActor :type "Actor Object Reference") (OtherComp :type "PrimitiveComponent Object Reference") (OtherBodyIndex :type Integer) (bFromSweep :type Boolean) (SweepResult :type "HitResult Structure (by ref)"))
  (bind _returnvalue (`GameplayStatics.GetPlayerPawn` 0))
  (if (== OtherActor _returnvalue)
    (bind _asplayer_character (cast `/Game/BluePrints/PlayerCharacter` _returnvalue))
    (`CharacterMovementComponent.SetMovementMode` (`Character.CharacterMovement` _asplayer_character) "MOVE_Flying" 0)
    (set `/Game/BluePrints/PlayerCharacter.CanFly` true _asplayer_character)))

(event `self.Box.OnComponentEndOverlap`
  (params (OverlappedComponent :type "PrimitiveComponent Object Reference") (OtherActor :type "Actor Object Reference") (OtherComp :type "PrimitiveComponent Object Reference") (OtherBodyIndex :type Integer))
  (bind _returnvalue (`GameplayStatics.GetPlayerPawn` 0))
  (if (== _returnvalue OtherActor)
    (bind _asplayer_character (cast `/Game/BluePrints/PlayerCharacter` _returnvalue))
    (`CharacterMovementComponent.SetMovementMode` (`Character.CharacterMovement` _asplayer_character) "MOVE_Walking" 0)
    (set `/Game/BluePrints/PlayerCharacter.CanFly` false _asplayer_character)))

(fn `UserConstructionScript`)