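; Staircase actor that teleports the player, apparently to move them downstairs to a linked Target staircase.
; Box overlap toggles ladder availability; while available, Tick polls the player's Temp flag and calls Use.
; Use teleports the player to Scene1, then after a delay to Scene2, and sets TeleportToTarget.
; Entering Box1 triggers a delayed teleport to Target's Scene2 if that flag is set, otherwise to Scene1; leaving Box1 clears it.
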(event `self.ReceiveTick`
  (params (DeltaSeconds :type "Float (single-precision)"))
  (set `self.Delta Time` DeltaSeconds)
  (if (`self.IsAvailable`)
    (bind _asplayer_character (cast `/Game/BluePrints/PlayerCharacter` (`GameplayStatics.GetPlayerPawn` 0)))
    (if (`/Game/BluePrints/PlayerCharacter.Temp` _asplayer_character)
      (`self.Use`)
      (set `/Game/BluePrints/PlayerCharacter.Temp` false _asplayer_character))))

(event `self.Box1.OnComponentBeginOverlap`
  (params (OverlappedComponent :type "PrimitiveComponent Object Reference") (OtherActor :type "Actor Object Reference") (OtherComp :type "PrimitiveComponent Object Reference") (OtherBodyIndex :type Integer) (bFromSweep :type Boolean) (SweepResult :type "HitResult Structure (by ref)"))
  (bind _returnvalue (`GameplayStatics.GetPlayerPawn` 0))
  (if (== OtherActor _returnvalue)
    (bind _asplayer_character (cast `/Game/BluePrints/PlayerCharacter` _returnvalue))
    (`KismetSystemLibrary.Delay` (`self.Delay`))
    (if (`self.TeleportToTarget`)
      (`self.K2_SetActorLocation` _asplayer_character (`SceneComponent.K2_GetComponentLocation` (`/Game/BluePrints/StaircaseToUpstair.Scene2` (`self.Target`))) false true)
      (else
        (`self.K2_SetActorLocation` _asplayer_character (`SceneComponent.K2_GetComponentLocation` (`self.Scene1`)) false true)))))

(event `self.Box1.OnComponentEndOverlap`
  (params (OverlappedComponent :type "PrimitiveComponent Object Reference") (OtherActor :type "Actor Object Reference") (OtherComp :type "PrimitiveComponent Object Reference") (OtherBodyIndex :type Integer))
  (if (== OtherActor (`GameplayStatics.GetPlayerPawn` 0))
    (set `self.TeleportToTarget` false)))

(event `self.Box.OnComponentBeginOverlap`
  (params (OverlappedComponent :type "PrimitiveComponent Object Reference") (OtherActor :type "Actor Object Reference") (OtherComp :type "PrimitiveComponent Object Reference") (OtherBodyIndex :type Integer) (bFromSweep :type Boolean) (SweepResult :type "HitResult Structure (by ref)"))
  (bind _returnvalue (`GameplayStatics.GetPlayerPawn` 0))
  (if (== OtherActor _returnvalue)
    (bind _asplayer_character (cast `/Game/BluePrints/PlayerCharacter` _returnvalue))
    (bind _output_get (set `/Game/BluePrints/PlayerCharacter.IsAbleToUseLadder` true _asplayer_character))
    (set `self.IsAvailable` _output_get)))

(event `self.Box.OnComponentEndOverlap`
  (params (OverlappedComponent :type "PrimitiveComponent Object Reference") (OtherActor :type "Actor Object Reference") (OtherComp :type "PrimitiveComponent Object Reference") (OtherBodyIndex :type Integer))
  (bind _returnvalue (`GameplayStatics.GetPlayerPawn` 0))
  (if (== OtherActor _returnvalue)
    (bind _asplayer_character (cast `/Game/BluePrints/PlayerCharacter` _returnvalue))
    (bind _output_get (set `/Game/BluePrints/PlayerCharacter.IsAbleToUseLadder` false _asplayer_character))
    (set `self.IsAvailable` _output_get)))

(event `Use`
  (bind _asplayer_character (cast `/Game/BluePrints/PlayerCharacter` (`GameplayStatics.GetPlayerPawn` 0)))
  (`self.K2_SetActorLocation` _asplayer_character (`SceneComponent.K2_GetComponentLocation` (`self.Scene1`)) false true)
  (`KismetSystemLibrary.Delay` 1.0)
  (`self.K2_SetActorLocation` _asplayer_character (`SceneComponent.K2_GetComponentLocation` (`self.Scene2`)) false true)
  (set `self.TeleportToTarget` true))

(fn `UserConstructionScript`)