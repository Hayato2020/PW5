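; Letter is an interactable that shows its Message text to the player in a MessageDialog widget.
; Overlapping its Sphere registers it as the PlayerCharacter's Letter and enables interaction, while leaving only clears the interaction flag.
; Display creates the widget, stores it on the character cached at overlap and adds it to the viewport.
; A Displaying flag blocks repeat displays and is never reset here.
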(event `self.Sphere.OnComponentBeginOverlap`
  (params (OverlappedComponent :type "PrimitiveComponent Object Reference") (OtherActor :type "Actor Object Reference") (OtherComp :type "PrimitiveComponent Object Reference") (OtherBodyIndex :type Integer) (bFromSweep :type Boolean) (SweepResult :type "HitResult Structure (by ref)"))
  (bind _returnvalue (`GameplayStatics.GetPlayerPawn` 0))
  (if (== OtherActor _returnvalue)
    (bind _asplayer_character (cast `/Game/BluePrints/Player/PlayerCharacter` _returnvalue))
    (set `/Game/BluePrints/Player/PlayerCharacter.Letter` self _asplayer_character)
    (set `/Game/BluePrints/Player/PlayerCharacter.IsAbleToInteract` true _asplayer_character)))

(event `Display`
  (if (not (`self.Displaying`))
    (bind _returnvalue (`|CreateWidget` "/Game/BluePrints/MessageDialog.MessageDialog_C"))
    (set `/Game/BluePrints/MessageDialog.Message` (`self.Message`) _returnvalue)
    (bind _output_get (set `/Game/BluePrints/Player/PlayerCharacter.MessageDialog` _returnvalue (stale `self.Sphere.OnComponentBeginOverlap` _asplayer_character)))
    (`UserWidget.AddToViewport` _output_get 0)
    (set `self.Displaying` true)))

(event `self.Sphere.OnComponentEndOverlap`
  (params (OverlappedComponent :type "PrimitiveComponent Object Reference") (OtherActor :type "Actor Object Reference") (OtherComp :type "PrimitiveComponent Object Reference") (OtherBodyIndex :type Integer))
  (bind _returnvalue (`GameplayStatics.GetPlayerPawn` 0))
  (if (== OtherActor _returnvalue)
    (bind _asplayer_character (cast `/Game/BluePrints/Player/PlayerCharacter` _returnvalue))
    (set `/Game/BluePrints/Player/PlayerCharacter.IsAbleToInteract` false _asplayer_character)))

(fn `UserConstructionScript`)